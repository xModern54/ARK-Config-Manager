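; Game mode for a config selector menu that opens registration, a stale-save error or the main config UI, based on save existence and optional version check.
; It routes config picks to switching or the template editor and shows queued alerts one at a time.
; A save-backed leveling system loads XP at BeginPlay, saves on EndPlay, maps levels to shader colors and sends Discord messages on level-up.
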(event Custom|AdapApp
  (bind _returnvalue (Game|GetPlayerController 0))
  (bind _returnvalue_2 (Settings|GetGameUserSettings))
  (Class|GameUserSettings|SetFullscreenMode _returnvalue_2 "Windowed")
  (Class|GameUserSettings|ApplyNonResolutionSettings _returnvalue_2)
  (Class|GameUserSettings|SaveSettings _returnvalue_2)
  (bind _returnvalue_3 (Settings|GetGameUserSettings))
  (Class|GameUserSettings|SetScreenResolution _returnvalue_3 (Utilities|Struct|MakeIntPoint 1280 720))
  (Class|GameUserSettings|ApplyResolutionSettings _returnvalue_3 true)
  (Class|GameUserSettings|SaveSettings _returnvalue_3)
  (Input|SetInputModeUIOnly _returnvalue 0 "DoNotLock")
  (Variables|/Script/Engine.PlayerController|SetbShowMouseCursor _returnvalue true)
  (Development|ExecuteConsoleCommand "t.maxfps 60" _returnvalue))

(event Custom|SET%20VAR
  (params (CurretID :type Integer) (Is%20Custom%20Bool :type Boolean) (b%20For%20Template :type Boolean))
  (if b%20For%20Template
    (CallFunction|ConstructConfigData CurretID Is%20Custom%20Bool)
    (else
      (Default|TriggerSwitchConfig (Variables|Default|GetNewVar_1) CurretID Is%20Custom%20Bool)
      (Development|PrintString (Utilities|String|ToString(Integer) CurretID))
      (if Is%20Custom%20Bool
        (Development|PrintString "custom cfg")))))

(event Custom|LevelingSysten_Shutdown
  (bind _savename (Variables|Default|GetSaveName))
  (bind _returnvalue (SaveGame|LoadGamefromSlot _savename))
  (bind _ask2_leveling (Utilities|Casting|CastToK2_Leveling _returnvalue))
  (Variables|/Game/K2_Leveling.K2_Leveling_C|SetLevel _ask2_leveling (Variables|level|Getlevel))
  (Variables|/Game/K2_Leveling.K2_Leveling_C|SetPlayerXP _ask2_leveling (Variables|level|GetXP))
  (SaveGame|SaveGametoSlot _ask2_leveling _savename))

(event Custom|ConstructConfigData
  (params (Config%20ID :type Integer) (Is%20custom? :type Boolean))
  (Widget|RemovefromParent (Variables|Default|GetNewVar_2))
  (if Is%20custom?
    (bind _returnvalue (SaveGame|LoadGamefromSlot "Own Configs"))
    (bind _asown_configs (Utilities|Casting|CastToOwnConfigs _returnvalue))
    (bind _returnvalue_2 (UserInterface|CreateWidget "/Game/WBP/WBP_ConfigEditor.WBP_ConfigEditor_C" (Game|GetPlayerController 0) (.ConfigData (Utilities|Struct|BreakConfigARKScruct (Utilities|Array|Get(acopy) (Variables|/Game/OwnConfigs.OwnConfigs_C|GetOwnConfigs _asown_configs) Config%20ID))) (Utilities|String|ToString(Text) (.Name (Utilities|Struct|BreakConfigARKScruct (Utilities|Array|Get(acopy) (Variables|/Game/OwnConfigs.OwnConfigs_C|GetOwnConfigs _asown_configs) Config%20ID)))) (Utilities|String|ToString(Text) (.Discription (Utilities|Struct|BreakConfigARKScruct (Utilities|Array|Get(acopy) (Variables|/Game/OwnConfigs.OwnConfigs_C|GetOwnConfigs _asown_configs) Config%20ID))))))
    (UserInterface|Viewport|AddtoViewport _returnvalue_2 0)
    (else
      (bind _returnvalue_3 (SaveGame|LoadGamefromSlot "UserSetting"))
      (bind _assetting_save (Utilities|Casting|CastToSettingSave _returnvalue_3))
      (bind _returnvalue_4 (UserInterface|CreateWidget "/Game/WBP/WBP_ConfigEditor.WBP_ConfigEditor_C" (Game|GetPlayerController 0) (.ConfigData (Utilities|Struct|BreakConfigARKScruct (Utilities|Array|Get(acopy) (Variables|/Game/SettingSave.SettingSave_C|GetConfigsArr _assetting_save) Config%20ID))) (Utilities|String|ToString(Text) (.Name (Utilities|Struct|BreakConfigARKScruct (Utilities|Array|Get(acopy) (Variables|/Game/SettingSave.SettingSave_C|GetConfigsArr _assetting_save) Config%20ID)))) (Utilities|String|ToString(Text) (.Discription (Utilities|Struct|BreakConfigARKScruct (Utilities|Array|Get(acopy) (Variables|/Game/SettingSave.SettingSave_C|GetConfigsArr _assetting_save) Config%20ID))))))
      (UserInterface|Viewport|AddtoViewport _returnvalue_4 0))))

(event Custom|OpenSelTemplateUI
  (bind _returnvalue (UserInterface|CreateWidget "/Game/WBP/WBP_SelectTemplate.WBP_SelectTemplate_C" (Game|GetPlayerController 0)))
  (bind _output_get (Variables|Default|SetNewVar_2 _returnvalue))
  (UserInterface|Viewport|AddtoViewport _output_get 0))

(event Custom|OpenMainUI
  (bind _returnvalue (UserInterface|CreateWidget "/Game/WBP/WBP_Config.WBP_Config_C" 0 true true))
  (bind _output_get (Variables|Default|SetNewVar_1 _returnvalue))
  (UserInterface|Viewport|AddtoViewport _output_get 0))

(event Custom|CustomEvent_0
  (CallFunction|NotifyEntryEvent (Utilities|String|Append (Utilities|String|ToString(Float) (Class|KismetMathLibrary|GetTotalMilliseconds (- (Math|DateTime|Now) (Variables|Default|GetTime)))) " ms")))

(event Custom|InitLevelingSystem
  (bind _savename (Variables|Default|GetSaveName))
  (bind _returnvalue (SaveGame|DoesSaveGameExist _savename))
  (if _returnvalue
    (bind _returnvalue_2 (SaveGame|LoadGamefromSlot _savename))
    (bind _ask2_leveling (Utilities|Casting|CastToK2_Leveling _returnvalue_2))
    (Variables|level|Setlevel (Variables|/Game/K2_Leveling.K2_Leveling_C|GetLevel _ask2_leveling))
    (Variables|level|SetXP (Variables|/Game/K2_Leveling.K2_Leveling_C|GetPlayerXP _ask2_leveling))
    (else
      (bind _returnvalue_3 (SaveGame|CreateSaveGameObject "/Game/K2_Leveling.K2_Leveling_C"))
      (Variables|/Game/K2_Leveling.K2_Leveling_C|SetPlayerXP _returnvalue_3 0.0)
      (Variables|/Game/K2_Leveling.K2_Leveling_C|SetLevel _returnvalue_3 0)
      (SaveGame|SaveGametoSlot _returnvalue_3 _savename)
      (Variables|level|SetXP 0.0)
      (Variables|level|Setlevel 0))))

(event Custom|CreateDelConfigs
  (bind _returnvalue (UserInterface|CreateWidget "/Game/WBP/WBP_DeleteConfigs.WBP_DeleteConfigs_C" (Game|GetPlayerController 0)))
  (bind _output_get (Variables|Default|SetNewVar_3 _returnvalue))
  (UserInterface|Viewport|AddtoViewport _output_get 0))

(event Custom|Register
  (CallFunction|AdapApp)
  (bind _returnvalue (UserInterface|CreateWidget "/Game/WBP/WBP_Trail_New.WBP_Trail_New_C" (Game|GetPlayerController 0)))
  (UserInterface|Viewport|AddtoViewport _returnvalue 0)
  (SaveGame|DeleteGameinSlot "UserSetting")
  (SaveGame|DeleteGameinSlot "Trail"))

(event Custom|refresh%20configs
  (Default|Refresh (Variables|Default|GetNewVar_3)))

(event EventBeginPlay
  (bind _returnvalue (Game|GetPlayerController 0))
  (bind _returnvalue_2 (Game|GetPlayerController 0))
  (bind _returnvalue_3 (Game|GetPlayerController 0))
  (Utilities|FlowControl|Sequence
    (:then_0
      (Variables|Default|SetTime (Math|DateTime|Now))
      (Utilities|FlowControl|Sequence
        (:then_0
          (bind _returnvalue_4 (UserInterface|CreateWidget "/Game/WBP/Backdrop_Selector.Backdrop_Selector_C" _returnvalue))
          (UserInterface|Viewport|AddtoViewport _returnvalue_4 0)
          (bind _returnvalue_5 (SaveGame|DoesSaveGameExist "bSecondLaunch"))
          (if _returnvalue_5
            (if (Variables|Default|GetbKillOldSaves)
              (bind _returnvalue_6 (SaveGame|LoadGamefromSlot "bSecondLaunch"))
              (bind _asb_second_launch (Utilities|Casting|CastTobSecondLaunch _returnvalue_6))
              (if (Utilities|Enum|Equal(Enum) (Variables|/Game/bSecondLaunch.bSecondLaunch_C|GetValidVersion _asb_second_launch) (Variables|Default|GetBuildVersionCurrent))
                (bind _returnvalue_7 (Settings|GetGameUserSettings :!label _label))
                (Class|GameUserSettings|ApplyNonResolutionSettings _returnvalue_7)
                (Class|GameUserSettings|ApplyResolutionSettings _returnvalue_7 false)
                (Class|GameUserSettings|LoadSettings _returnvalue_7 false)
                (Input|SetInputModeUIOnly _returnvalue_2 0 "DoNotLock")
                (Variables|/Script/Engine.PlayerController|SetbShowMouseCursor _returnvalue_2 true)
                (bind _returnvalue_8 (UserInterface|CreateWidget "/Game/WBP/WBP_Config.WBP_Config_C" (Game|GetPlayerController 0)))
                (bind _output_get (Variables|Default|SetNewVar_1 _returnvalue_8))
                (UserInterface|Viewport|AddtoViewport _output_get 0)
                (bind _returnvalue_9 (SaveGame|LoadGamefromSlot "UserSetting"))
                (bind _assetting_save (Utilities|Casting|CastToSettingSave _returnvalue_9))
                (Variables|Default|SetbDisableNotify (Variables|/Game/SettingSave.SettingSave_C|GetbDisableNotifySystem _assetting_save))
                (else
                  (bind _returnvalue_10 (UserInterface|CreateWidget "/Game/WBP/WBP_Error.WBP_Error_C" (Game|GetPlayerController 0) "Ошибка сохранений" "Сохранения устарели, необходимо пройти регистрацию заново. " false true))
                  (UserInterface|Viewport|AddtoViewport _returnvalue_10 0)))
              (else
                (goto _label)))
            (else
              (CallFunction|AdapApp)
              (bind _returnvalue_11 (UserInterface|CreateWidget "/Game/WBP/WBP_Trail_New.WBP_Trail_New_C" _returnvalue))
              (UserInterface|Viewport|AddtoViewport _returnvalue_11 0)
              (SaveGame|DeleteGameinSlot "UserSetting")
              (SaveGame|DeleteGameinSlot "Trail"))))
        (:then_1
          (Input|SetInputModeUIOnly _returnvalue_3 0 "DoNotLock")
          (Variables|/Script/Engine.PlayerController|SetbShowMouseCursor _returnvalue_3 true))))
    (:then_1
      (CallFunction|InitLevelingSystem))))

(event EventTick
  (params (DeltaSeconds :type Float%20%28single-precision%29)))

(event EventAddNotifyInterface
  (params (Header :type Text) (Text :type Text) (Duration :type Float%20%28single-precision%29))
  (bind _notify_queue (Variables|Default|GetNotify_Queue))
  (bind _output (Utilities|Array|Get(acopy) _notify_queue))
  (bind (_header _text _duration) (Utilities|Struct|BreakSt_Alert _output))
  (if (not (Variables|Default|GetbDisableNotify))
    (Utilities|FlowControl|Delay 0.05)
    (Utilities|Array|Add (Variables|Default|GetNotify_Queue) (Utilities|Struct|MakeSt_Alert Header Text Duration))
    (if (not (Variables|Default|GetbAlertShowesNow)) :!label _label
      (if (not (== (Utilities|Array|Length _notify_queue) 0))
        (Variables|Default|SetbAlertShowesNow true)
        (bind _returnvalue (UserInterface|CreateWidget "/Game/Matchmaking/WBP/WBP_ServerAlert.WBP_ServerAlert_C" (Game|GetPlayerController 0) _duration _text _header))
        (UserInterface|Viewport|AddtoViewport _returnvalue 0)
        (Utilities|FlowControl|Delay (+ _duration 1.0))
        (Utilities|Array|RemoveIndex (Variables|Default|GetNotify_Queue))
        (Variables|Default|SetbAlertShowesNow false)
        (goto _label)))))

(event EventEndPlay
  (params (EndPlayReason :type EEndPlayReason%20Enum :default "Destroyed"))
  (CallFunction|LevelingSystenShutdown))

(fn ConstructionScript)

(fn OnRepIDtemp)

(fn NewFunction1)

(fn UpdateLevel
  (return false))

(fn LevelUpdate
  (switch int (Variables|level|Getlevel)
    (:0
      (LocalVariables|SetXpToNextLevel (Variables|Default|Getlevel1xp)))
    (:1
      (LocalVariables|SetXpToNextLevel (Variables|Default|Getlevel2xp)))
    (:2
      (LocalVariables|SetXpToNextLevel (Variables|Default|Getlevel3xp)))
    (:3
      (LocalVariables|SetXpToNextLevel (Variables|Default|Getlevel4xp)))
    (:4
      (LocalVariables|SetXpToNextLevel (Variables|Default|Getlevel5xp))))
  (if (>= (Variables|level|GetXP) (LocalVariables|GetXpToNextLevel))
    (if (== (Variables|level|GetMaxLevel) (Variables|level|Getlevel))
      _
      (else
        (bind _output_get (Variables|level|Setlevel (+ (Variables|level|Getlevel) 1)))
        (switch int (Variables|level|Getlevel)
          (:0
            _)
          (:1
            (LocalVariables|Settemp "Green")
            (CallFunction|FunctionSendFuckingDcMEssage "Leveling Up!" "NewEnumerator5" (Utilities|Array|MakeArray (Utilities|Struct|MakeDiscordField "New Level" (Utilities|String|ToString(Integer) (Variables|level|Getlevel)) true) (Utilities|Struct|MakeDiscordField "Available Shader" (LocalVariables|Gettemp) true)) :!label _label))
          (:2
            (LocalVariables|Settemp "Blue")
            (goto _label))
          (:3
            (LocalVariables|Settemp "Yellow")
            (goto _label))
          (:4
            (LocalVariables|Settemp "Purpule")
            (goto _label))
          (:5
            (LocalVariables|Settemp "Red")
            (goto _label))))))
  (return _output_get))

(fn GetIsEnglish
  (return (Variables|Default|GetKangIsEng)))

(fn GetIsEngLan
  (return (Variables|Default|GetKangIsEng)))

(fn GetLevel
  (return (Variables|level|Getlevel)))

(fn GetShaderFluxColor
  (switch int (Variables|level|Getlevel)
    (:0
      (LocalVariables|SetFluxColor (Utilities|Struct|MakeLinearColor 0.0 0.647565 1.0 1.0)))
    (:1
      (LocalVariables|SetFluxColor (Utilities|Struct|MakeLinearColor 0.015102 1.0 0.0 1.0)))
    (:2
      (LocalVariables|SetFluxColor (Utilities|Struct|MakeLinearColor 0.0 0.012573 1.0 1.0)))
    (:3
      (LocalVariables|SetFluxColor (Utilities|Struct|MakeLinearColor 1.0 0.902294 0.021552 1.0)))
    (:4
      (LocalVariables|SetFluxColor (Utilities|Struct|MakeLinearColor 1.0 0.0 0.577788 1.0)))
    (:5
      (LocalVariables|SetFluxColor (Utilities|Struct|MakeLinearColor 1.0 0.0 0.014842 1.0))))
  (return (LocalVariables|GetFluxColor) "FluxColor"))

(fn GetXp
  (return (Variables|level|GetXP)))

(fn PlayerReciveXP
  (params (Amount :type Float%20%28single-precision%29))
  (Variables|level|SetXP (+ (Variables|level|GetXP) Amount))
  (bind _currentlevel (CallFunction|LevelUpdate))
  (return _currentlevel))